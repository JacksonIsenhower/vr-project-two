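; Text render actor for the basketball game that displays the highest score the VR player has reached.
; Every Tick it casts player pawn 0 to VRPawn and compares the pawn's Score with its own HighScore variable.
; When the score is higher, it rewrites the "High Score:" text and stores the new value, with no save to disk.
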(event `self.ReceiveTick`
  (params (DeltaSeconds :type "Float (single-precision)"))
  (bind _asvrpawn (cast `/Game/VRTemplate/Blueprints/VRPawn` (`GameplayStatics.GetPlayerPawn` 0)))
  (bind _score (`/Game/VRTemplate/Blueprints/VRPawn.Score` _asvrpawn))
  (if (> _score (`self.HighScore`))
    (`TextRenderComponent.K2_SetText` (`self.TextRender`) (`KismetTextLibrary.Conv_StringToText` (`KismetStringLibrary.Concat_StrStr` "High Score: " (`KismetStringLibrary.Conv_IntToString` _score))))
    (set `self.HighScore` _score)))

(fn `UserConstructionScript`)