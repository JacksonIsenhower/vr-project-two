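; A text render actor that shows the current round time from the player's VR pawn in the world.
; Each tick it casts player pawn 0 to VRPawn and, while RoundComplete is false, sets its text to "Time:" followed by the pawn's Timer.
; Once the round completes it stops updating, so the last written time stays displayed.
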(event `self.ReceiveTick`
  (params (DeltaSeconds :type "Float (single-precision)"))
  (bind _asvrpawn (cast `/Game/VRTemplate/Blueprints/VRPawn` (`GameplayStatics.GetPlayerPawn` 0)))
  (if (not (`/Game/VRTemplate/Blueprints/VRPawn.RoundComplete` _asvrpawn))
    (`TextRenderComponent.K2_SetText` (`self.TextRender`) (`KismetTextLibrary.Conv_StringToText` (`KismetStringLibrary.Concat_StrStr` "Time: " (`KismetStringLibrary.Conv_IntToString` (`/Game/VRTemplate/Blueprints/VRPawn.Timer` _asvrpawn)))))))

(fn `UserConstructionScript`
  (`parent.UserConstructionScript`))